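; BP_CubeGenerator is a spawner actor that periodically produces BP_DropCube actors until a linked pressure plate stops it.
; BeginPlay starts a looping timer that spawns a cube at the SpawnLocation component, adjusting for collisions but always spawning.
; If BindedPressurePlate is valid, its activation event clears the timer, permanently halting generation since nothing restarts it.
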(event Custom|GenerateNewCube
  (Game|SpawnActorfromClass "/Game/PhysicsActors/BP_DropCube.BP_DropCube_C" (Transformation|GetWorldTransform (Variables|Default|GetSpawnLocation)) "AdjustIfPossibleButAlwaysSpawn" "MultiplyWithRoot" 0 0))

(event Custom|StopGenerate
  (Utilities|Time|ClearandInvalidateTimerbyHandle (Variables|Default|GetGenerateTimerHandle)))

(event EventBeginPlay
  (bind _returnvalue (Utilities|Time|SetTimerbyEvent (delegate Custom|GenerateNewCube) 5.0 true))
  (Variables|Default|SetGenerateTimerHandle _returnvalue)
  (Utilities|IsValid (Variables|Default|GetBindedPressurePlate)
    (:Is%20Valid
      (EventDispatchers|BindEventtoOnPressurePlateActivated (Variables|Default|GetBindedPressurePlate) (delegate Custom|StopGenerate)))))

(fn ConstructionScript)