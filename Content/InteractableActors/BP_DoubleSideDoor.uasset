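; BP_DoubleSideDoor is an interactable double door that opens when the interacting actor's inventory holds the required item.
; Interact consumes that item, then enables physics on both leaves and binds each to its base through axis constraint components, so the door swings physically rather than animating.
; A missing item or inventory only prints a failure message.
; Once open, CanInteract returns false, blocking further interaction.
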(event EventBeginPlay)

(event Collision|EventActorBeginOverlap
  (params (OtherActor :type Actor%20Object%20Reference)))

(event EventTick
  (params (DeltaSeconds :type Float%20%28single-precision%29)))

(event EventInteract
  (params (InHandItem :type Item%20Object%20Reference) (FromActor :type Actor%20Object%20Reference))
  (bind _returnvalue (Class|InventorySystemInterface|GetInventoryComponent(Message) FromActor))
  (Utilities|IsValid _returnvalue
    (:Is%20Valid
      (bind _returnvalue_2 (Class|InventoryComponent|ContainsItem _returnvalue (Variables|Default|GetNeededItemName)))
      (if (!= _returnvalue_2 -1)
        (Class|InventoryComponent|RemoveItembyIndex _returnvalue _returnvalue_2)
        ;[1 1 1] 打开门
        (Physics|SetSimulatePhysics (Variables|Default|GetDoorRight) true)
        (Class|PhysicsConstraintComponent|SetConstrainedComponents (Variables|Default|GetLeftDoorAxis) (Variables|Default|GetDoorLeft) "None" (Variables|Default|GetBaseLeft) "None")
        (Class|PhysicsConstraintComponent|SetConstrainedComponents (Variables|Default|GetRightDoorAxis) (Variables|Default|GetDoorRight) "None" (Variables|Default|GetBaseRight) "None")
        (Variables|Default|SetbIsOpen true)
        (else
          ;[1 1 1] 发出提示
          (Development|PrintString "开门失败" :!label _label))))
    (:Is%20Not%20Valid
      (goto _label))))

(fn ConstructionScript)

(fn CanInteract
  (params (InHandItem :type Item%20Object%20Reference) (FromActor :type Actor%20Object%20Reference))
  (return (not (Variables|Default|GetbIsOpen))))

(fn GetInteractText
  (return "打开门"))

(fn ShouldUpdate
  (return false))