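; BP_Button is an interactable physical button that calls clicked and released events when used.
; Interact enables physics on the button mesh and shifts a PhysicsConstraint linear position target to move it.
; Chained timers then return the target to rest, signal the release and switch simulation off again, so physics runs only during a press.
; CanInteract blocks re-use while the press is active.
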(event Custom|ResetButton
  (Class|PhysicsConstraintComponent|SetLinearPositionTarget (Variables|Default|GetPhysicsConstraint) (Math|Vector|MakeVector 0.0 0.0 0.0))
  (Class|PrimitiveComponent|WakeRigidBody (Variables|Default|GetButton) "None")
  (Utilities|Time|SetTimerbyEvent (delegate Custom|ResetSimulatePhysics) 0.3)
  (Default|CallOnButtonReleased))

(event Custom|ResetSimulatePhysics
  (Physics|SetSimulatePhysics (Variables|Default|GetButton) false)
  (Variables|Default|SetIsActive false))

(event EventBeginPlay)

(event Collision|EventActorBeginOverlap
  (params (OtherActor :type Actor%20Object%20Reference)))

(event EventTick
  (params (DeltaSeconds :type Float%20%28single-precision%29)))

(event EventInteract
  (params (InHandItem :type Item%20Object%20Reference) (FromActor :type Actor%20Object%20Reference))
  (Variables|Default|SetIsActive true)
  (Physics|SetSimulatePhysics (Variables|Default|GetButton) true)
  (Class|PhysicsConstraintComponent|SetLinearPositionTarget (Variables|Default|GetPhysicsConstraint) (Math|Vector|MakeVector 0.0 0.0 3.0))
  (Class|PrimitiveComponent|WakeRigidBody (Variables|Default|GetButton) "None")
  (Default|CallOnButtonClicked)
  (Utilities|Time|SetTimerbyEvent (delegate Custom|ResetButton) 1.0))

(fn ConstructionScript)

(fn CanInteract
  (params (InHandItem :type Item%20Object%20Reference) (FromActor :type Actor%20Object%20Reference))
  (return (not (Variables|Default|GetIsActive))))

(fn GetInteractText
  (return (Variables|Default|GetInteractText)))

(fn ShouldUpdate
  (return false))