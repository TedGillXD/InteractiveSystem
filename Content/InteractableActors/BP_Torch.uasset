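; BP_Torch is a world pickup that gives the first-person player a torch.
; On Interact it sets the child actor class of BP_FirstPersonCharacter to BP_Torch_Picked, then destroys itself.
; Interaction is open to any Character with a Chinese "get illuminator" prompt, but only BP_FirstPersonCharacter can complete the pickup.
; ShouldUpdate always returns false.
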(event EventBeginPlay)

(event Collision|EventActorBeginOverlap
  (params (OtherActor :type Actor%20Object%20Reference)))

(event EventTick
  (params (DeltaSeconds :type Float%20%28single-precision%29)))

(event EventInteract
  (params (InHandItem :type Item%20Object%20Reference) (FromActor :type Actor%20Object%20Reference))
  (bind _asbp_first_person_character (Utilities|Casting|CastToBP_FirstPersonCharacter FromActor))
  (ChildActorComponent|SetChildActorClass (Variables|/Game/FirstPerson/Blueprints/BP_FirstPersonCharacter.BP_FirstPersonCharacter_C|GetChildActor _asbp_first_person_character) "/Game/NormalActors/BP_Torch_Picked.BP_Torch_Picked_C")
  (Actor|DestroyActor))

(fn ConstructionScript)

(fn CanInteract
  (params (InHandItem :type Item%20Object%20Reference) (FromActor :type Actor%20Object%20Reference))
  (return (Class|GameplayStatics|ObjectIsA FromActor "/Script/Engine.Character")))

(fn GetInteractText
  (return "获取照明器"))

(fn ShouldUpdate
  (return false))