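; Rotatable puzzle statue that adds 90 degrees to its target yaw each time its bound button is clicked.
; Tick turns the Cone toward that angle, scaling FInterpTo speed by remaining angle and delta time to get a fixed step per frame.
; On settling at the unwrapped Target angle, it asks BP_FirstPersonGameMode once to check statue status.
; IsInRightRotation compares the angle modulo 360 to Target.
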(event Custom|BindButtonClicked
  (Variables|Default|SetTargetDegree (+ (Variables|Default|GetTargetDegree) 9e+01))
  (Development|PrintString (Utilities|String|ToString(Float) (Variables|Default|GetTargetDegree))))

(event EventBeginPlay
  (EventDispatchers|BindEventtoOnButtonClicked (Variables|Default|GetBindButton) (delegate Custom|BindButtonClicked)))

(event EventTick
  (params (DeltaSeconds :type Float%20%28single-precision%29))
  (bind _cone (Variables|Default|GetCone))
  (bind _relativerotation (Variables|/Script/Engine.SceneComponent|GetRelativeRotation _cone))
  (if (Math|Float|NearlyEqual(Float) (Variables|Default|GetCurrentDegree) (Variables|Default|GetTargetDegree) 1e-06)
    (if (Math|Float|NearlyEqual(Float) (Variables|Default|GetCurrentDegree) (Variables|Default|GetTarget) 1e-06)
      (Utilities|FlowControl|DoOnce false :!label _label
        (:Completed
          (bind _asbp_first_person_game_mode (Utilities|Casting|CastToBP_FirstPersonGameMode (Game|GetGameMode)))
          (Class|InteractiveSystemGameMode|CheckStatueStatus _asbp_first_person_game_mode))))
    (else
      (Utilities|FlowControl|Sequence
        (:then_0
          (goto _label Reset))
        (:then_1
          (Transformation|SetRelativeRotation _cone (Math|Rotator|MakeRotator (.roll _relativerotation) (.pitch _relativerotation) (Math|Interpolation|FInterpTo (Variables|Default|GetCurrentDegree) (Variables|Default|GetTargetDegree) DeltaSeconds (CallFunction|GetInterpTime))) false false)
          (Variables|Default|SetCurrentDegree (Math|Interpolation|FInterpTo (Variables|Default|GetCurrentDegree) (Variables|Default|GetTargetDegree) DeltaSeconds (CallFunction|GetInterpTime))))))))

(fn ConstructionScript)

(fn IsinRightRotation
  (return (Math|Float|NearlyEqual(Float) (Variables|Default|GetTarget) (Math|Float|%(Float) (Variables|Default|GetCurrentDegree) 3.6e+02) 1e-06)))

(fn GetInterpTime
  (return (/ (LocalVariables|GetConstant) (* (- (Variables|Default|GetTargetDegree) (Variables|Default|GetCurrentDegree)) (Utilities|Time|GetWorldDeltaSeconds)))))